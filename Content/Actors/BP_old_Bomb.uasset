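; An older bomb actor that deals damage to the third-person player character.
; BeginPlay starts a one-shot timer, and a separate Explode event activates the particle system, hides the mesh and stops its physics.
; Damage is independent of Explode: any overlap with the Sphere casts to BP_ThirdPersonCharacter and calls GetDamage with a fixed amount.
; The timer shows no bound event, and the actor is never destroyed here.
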(event `self.ReceiveBeginPlay`
  (`parent.ReceiveBeginPlay`)
  (`KismetSystemLibrary.K2_SetTimerDelegate` :`Time` 15.0))

(event `Explode`
  (bind _visualmesh (`self.VisualMesh`))
  (`ActorComponent.Activate` (`self.ParticleSystem`) false)
  (`SceneComponent.SetVisibility` _visualmesh false false)
  (`PrimitiveComponent.SetSimulatePhysics` _visualmesh false))

(event `self.Sphere.OnComponentBeginOverlap`
  (params (OverlappedComponent :type "PrimitiveComponent Object Reference") (OtherActor :type "Actor Object Reference") (OtherComp :type "PrimitiveComponent Object Reference") (OtherBodyIndex :type Integer) (bFromSweep :type Boolean) (SweepResult :type "HitResult Structure (by ref)"))
  (bind _asbp_third_person_character (cast `/Game/ThirdPerson/Blueprints/BP_ThirdPersonCharacter` OtherActor))
  (`/Game/ThirdPerson/Blueprints/BP_ThirdPersonCharacter.GetDamage` _asbp_third_person_character 3))

(fn `UserConstructionScript`)